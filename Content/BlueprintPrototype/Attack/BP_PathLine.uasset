(event EventBeginPlay
  (|CallParentFunction) ; This node is disabled and will not be called.\nDrag off pins to build functionality.
)

(event EventTick
  (params (DeltaSeconds :type Float%20%28single-precision%29))
  (|CallParentFunction DeltaSeconds) ; This node is disabled and will not be called.\nDrag off pins to build functionality.
)

(fn MakePath
  (params (Start%20Location :type Vector :default "0, 0, 0") (Target%20Location :type Vector :default "0, 0, 0") (Max%20Length :type Float%20%28double-precision%29) (Objects%20to%20Ignore :type Array%20of%20Actor%20Object%20References) (Clear%20Path%20Colour :type Linear%20Color%20Structure) (Failed%20Path%20Color :type Linear%20Color%20Structure))
  (bind _returnvalue (+ Target%20Location "0.000000,0.000000,0.000000"))
  (bind _returnvalue_2 (- _returnvalue Start%20Location))
  (bind _returnvalue_3 (Math|Vector|VectorLength _returnvalue_2))
  (bind _returnvalue_4 (> _returnvalue_3 Max%20Length))
  (bind _outhit (Collision|LineTraceByChannel Start%20Location _returnvalue "TraceTypeQuery1" false Objects%20to%20Ignore "ForOneFrame" true (Math|Color|SelectColor Failed%20Path%20Color Clear%20Path%20Colour _returnvalue_4) Failed%20Path%20Color))
  (return (not _returnvalue_4) (not (.bBlockingHit (Collision|BreakHitResult _outhit))) (.bBlockingHit (Collision|BreakHitResult _outhit)) (.Location (Collision|BreakHitResult _outhit))))